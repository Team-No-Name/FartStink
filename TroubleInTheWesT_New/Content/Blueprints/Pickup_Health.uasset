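; Health pickup actor that gives the WesTurner_FPS character one unit of whisky.
; On overlap it casts the other actor and, if CurrentWhisky is below MaxWhisky, increments it, plays a liquid sound at its own location and destroys itself.
; Other actors, or a player already at maximum whisky, leave the pickup in place.
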(event Collision|EventActorBeginOverlap
  (params (OtherActor :type Actor%20Object%20Reference))
  (bind _aswes_turner_fps (Utilities|Casting|CastToWesTurner_FPS OtherActor))
  (if (< (Variables|/Game/WesTurner_Character/WesTurner_FPS.WesTurner_FPS_C|GetCurrentWhisky _aswes_turner_fps) (Variables|/Game/WesTurner_Character/WesTurner_FPS.WesTurner_FPS_C|GetMaxWhisky _aswes_turner_fps))
    (bind _result (Math|Integer|IncrementInt (Variables|/Game/WesTurner_Character/WesTurner_FPS.WesTurner_FPS_C|GetCurrentWhisky _aswes_turner_fps))
      (:%20%20
        (Variables|/Game/WesTurner_Character/WesTurner_FPS.WesTurner_FPS_C|SetCurrentWhisky _aswes_turner_fps _result)
        (Audio|PlaySoundatLocation "/Game/assets/SoundFX/Sound_Cues/whiskey_liquid.whiskey_liquid" (Transformation|GetWorldLocation (Variables|Default|GetDefaultSceneRoot)))
        (Actor|DestroyActor)))))

(fn ConstructionScript)