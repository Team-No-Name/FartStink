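; Dynamite pickup actor that adds one dynamite to the player's count.
; On overlap with a WesTurner_FPS, it increments CurrentDynamite only while below MaxDynamite.
; A successful pickup plays the FT_Run_Dirt_3 sound at the pickup's location and destroys the actor; otherwise it stays in the world.
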(event Collision|EventActorBeginOverlap
  (params (OtherActor :type Actor%20Object%20Reference))
  (bind _aswes_turner_fps (Utilities|Casting|CastToWesTurner_FPS OtherActor))
  (if (< (Variables|/Game/WesTurner_Character/WesTurner_FPS.WesTurner_FPS_C|GetCurrentDynamite _aswes_turner_fps) (Variables|/Game/WesTurner_Character/WesTurner_FPS.WesTurner_FPS_C|GetMaxDynamite _aswes_turner_fps))
    (bind _result (Math|Integer|IncrementInt (Variables|/Game/WesTurner_Character/WesTurner_FPS.WesTurner_FPS_C|GetCurrentDynamite _aswes_turner_fps))
      (:%20%20
        (Variables|/Game/WesTurner_Character/WesTurner_FPS.WesTurner_FPS_C|SetCurrentDynamite _aswes_turner_fps _result)
        (Audio|PlaySoundatLocation "/Game/assets/SoundFX/Footstep_Beta/FT_Run_Dirt_3.FT_Run_Dirt_3" (Transformation|GetWorldLocation (Variables|Default|GetDefaultSceneRoot)))
        (Actor|DestroyActor)))))

(fn ConstructionScript)