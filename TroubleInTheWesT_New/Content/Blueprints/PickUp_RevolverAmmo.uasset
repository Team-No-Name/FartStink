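; Revolver ammo pickup that refills the WesTurner_FPS character's revolver ammo on overlap.
; If that ammo is below max, it adds AmmoAmount, capped at the maximum, so any excess is lost.
; It then plays a sound at its location, destroys itself and prints the new count.
; At full ammo, the pickup stays in the world.
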(event Collision|EventActorBeginOverlap
  (params (OtherActor :type Actor%20Object%20Reference))
  (bind _aswes_turner_fps (Utilities|Casting|CastToWesTurner_FPS OtherActor))
  (if (< (Variables|/Game/WesTurner_Character/WesTurner_FPS.WesTurner_FPS_C|GetRevolverCurrentAmmo _aswes_turner_fps) (Variables|/Game/WesTurner_Character/WesTurner_FPS.WesTurner_FPS_C|GetRevolverMaxAmmo _aswes_turner_fps))
    (if (> (Variables|Default|GetAmmoAmount) (- (Variables|/Game/WesTurner_Character/WesTurner_FPS.WesTurner_FPS_C|GetRevolverMaxAmmo _aswes_turner_fps) (Variables|/Game/WesTurner_Character/WesTurner_FPS.WesTurner_FPS_C|GetRevolverCurrentAmmo _aswes_turner_fps)))
      (Variables|/Game/WesTurner_Character/WesTurner_FPS.WesTurner_FPS_C|SetRevolverCurrentAmmo _aswes_turner_fps (+ (Variables|/Game/WesTurner_Character/WesTurner_FPS.WesTurner_FPS_C|GetRevolverCurrentAmmo _aswes_turner_fps) (- (Variables|/Game/WesTurner_Character/WesTurner_FPS.WesTurner_FPS_C|GetRevolverMaxAmmo _aswes_turner_fps) (Variables|/Game/WesTurner_Character/WesTurner_FPS.WesTurner_FPS_C|GetRevolverCurrentAmmo _aswes_turner_fps))))
      (else
        (Variables|/Game/WesTurner_Character/WesTurner_FPS.WesTurner_FPS_C|SetRevolverCurrentAmmo _aswes_turner_fps (+ (Variables|/Game/WesTurner_Character/WesTurner_FPS.WesTurner_FPS_C|GetRevolverCurrentAmmo _aswes_turner_fps) (Variables|Default|GetAmmoAmount)))))
    (Audio|PlaySoundatLocation 0 (Transformation|GetWorldLocation (Variables|Default|GetDefaultSceneRoot)))
    (Actor|DestroyActor)
    (Development|PrintString (Utilities|String|ToString(Integer) (Variables|/Game/WesTurner_Character/WesTurner_FPS.WesTurner_FPS_C|GetRevolverCurrentAmmo _aswes_turner_fps)))))

(fn ConstructionScript)