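; BP_Dynamite is a spinning projectile explosive that detonates on a fuse or when damaged.
; When its projectile movement stops, it stops rotating, switches collision to physics simulation and explodes after a short delay.
; Taking any damage jumps straight to the explosion, which spawns particles and sound, applies full radial damage, draws a debug sphere and destroys the actor.
; It disables its own damageability before applying damage, so the blast cannot retrigger it.
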(event OnProjectileStop(ProjectileMovement)
  (params (ImpactResult :type Hit%20Result%20Structure%20%28by%20ref%29))
  (bind _returnvalue (Transformation|GetActorLocation))
  (bind _dynamite (Variables|Default|GetDynamite))
  (bind _explosiondamageradius (Variables|Default|GetExplosionDamageRadius))
  (bind _returnvalue_2 (Transformation|GetWorldLocation _dynamite))
  (Variables|/Script/Engine.RotatingMovementComponent|SetRotationRate (Variables|Default|GetRotatingMovement) "0, 0, 0")
  (Physics|SetSimulatePhysics (Variables|Default|GetCollision) true)
  (Utilities|FlowControl|Delay 2.0)
  (Effects|SpawnEmitteratLocation "/Game/WesTurner_Character/Particles/P_Explosion.P_Explosion" _returnvalue_2)
  (Variables|Actor|SetbCanBeDamaged false)
  (Audio|SpawnSoundatLocation "/Game/assets/SoundFX/Sound_Cues/explosion.explosion" _returnvalue_2)
  (Game|Damage|ApplyRadialDamage (Variables|Default|GetExplosionDamage) _returnvalue _explosiondamageradius "/Script/Engine.DamageType" 0 self 0 true "ECC_Visibility")
  (Rendering|Debug|DrawDebugSphere _returnvalue _explosiondamageradius 12 "(R=0.000000,G=0.188609,B=1.000000,A=1.000000)" 1.0)
  (Actor|DestroyActor))

(event Game|Damage|EventAnyDamage
  (params (Damage :type Float%20%28single-precision%29) (DamageType :type Damage%20Type%20Object%20Reference) (InstigatedBy :type Controller%20Object%20Reference) (DamageCauser :type Actor%20Object%20Reference))
  (bind _returnvalue (Transformation|GetActorLocation))
  (bind _dynamite (Variables|Default|GetDynamite))
  (bind _explosiondamageradius (Variables|Default|GetExplosionDamageRadius))
  (bind _returnvalue_2 (Transformation|GetWorldLocation _dynamite))
  (Effects|SpawnEmitteratLocation "/Game/WesTurner_Character/Particles/P_Explosion.P_Explosion" _returnvalue_2)
  (Variables|Actor|SetbCanBeDamaged false)
  (Audio|SpawnSoundatLocation "/Game/assets/SoundFX/Sound_Cues/explosion.explosion" _returnvalue_2)
  (Game|Damage|ApplyRadialDamage (Variables|Default|GetExplosionDamage) _returnvalue _explosiondamageradius "/Script/Engine.DamageType" 0 self 0 true "ECC_Visibility")
  (Rendering|Debug|DrawDebugSphere _returnvalue _explosiondamageradius 12 "(R=0.000000,G=0.188609,B=1.000000,A=1.000000)" 1.0)
  (Actor|DestroyActor))

(fn ConstructionScript)