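; BP_Shield is a thrown or launched projectile that deploys a shield where it hits.
; On Hit it stops its projectile movement, removes the FreezeTrap component and plays an explosion emitter at the collision location.
; It then spawns BP_ShieldSpawn at that location with zero rotation and destroys its collision component, leaving the actor itself in place.
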(event Collision|EventHit
  (params (MyComp :type Primitive%20Component%20Object%20Reference) (Other :type Actor%20Object%20Reference) (OtherComp :type Primitive%20Component%20Object%20Reference) (bSelfMoved :type Boolean) (HitLocation :type Vector :default "0, 0, 0") (HitNormal :type Vector :default "0, 0, 0") (NormalImpulse :type Vector :default "0, 0, 0") (Hit :type Hit%20Result%20Structure%20%28by%20ref%29))
  (bind _collision (Variables|Default|GetCollision))
  (bind _returnvalue (Transformation|GetWorldLocation _collision))
  (Components|Movement|StopMovementImmediately (Variables|Default|GetProjectileMovement))
  (Transformation|AttachComponentToComponent 0 "None" "KeepRelative" "KeepRelative" "KeepRelative" true)
  (Components|DestroyComponent (Variables|Default|GetFreezeTrap))
  (Effects|SpawnEmitteratLocation "/Game/WesTurner_Character/Particles/P_Explosion.P_Explosion" _returnvalue)
  (Game|SpawnActorfromClass "/Game/WesTurner_Character/Blueprints/Shield/BP_ShieldSpawn.BP_ShieldSpawn_C" (Math|Transform|MakeTransform _returnvalue) "Undefined" 0 0)
  (Components|DestroyComponent (Variables|Default|GetCollision)))

(fn ConstructionScript)