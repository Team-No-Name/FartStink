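; BP_Dynamite is a dynamite projectile that spins in flight and explodes after a short fuse once it comes to rest.
; When projectile movement stops, it halts the rotation, turns on physics for its collision and waits before detonating.
; Any damage it receives skips the fuse and detonates it immediately.
; Detonation spawns explosion particles and sound, applies full radial damage without falloff, then destroys the actor.
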(event OnProjectileStop(ProjectileMovement)
  (params (ImpactResult :type Hit%20Result%20Structure%20%28by%20ref%29))
  (bind _dynamite (Variables|Default|GetDynamite))
  (bind _returnvalue (Transformation|GetWorldLocation _dynamite))
  (Variables|/Script/Engine.RotatingMovementComponent|SetRotationRate (Variables|Default|GetRotatingMovement) "0, 0, 0")
  (Physics|SetSimulatePhysics (Variables|Default|GetCollision) true)
  (Utilities|FlowControl|Delay 2.0)
  (Effects|SpawnEmitteratLocation "/Game/WesTurner_Character/Particles/P_Explosion.P_Explosion" _returnvalue)
  (Audio|SpawnSoundatLocation "/Game/assets/SoundFX/Sound_Cues/explosion.explosion" _returnvalue)
  (Game|Damage|ApplyRadialDamage (Variables|Default|GetExplosionDamage) (Transformation|GetActorLocation) (Variables|Default|GetExplosionDamageRadius) "/Script/Engine.DamageType" 0 self 0 true "ECC_Visibility")
  (Actor|DestroyActor))

(event Game|Damage|EventAnyDamage
  (params (Damage :type Float%20%28single-precision%29) (DamageType :type Damage%20Type%20Object%20Reference) (InstigatedBy :type Controller%20Object%20Reference) (DamageCauser :type Actor%20Object%20Reference))
  (bind _dynamite (Variables|Default|GetDynamite))
  (bind _returnvalue (Transformation|GetWorldLocation _dynamite))
  (Effects|SpawnEmitteratLocation "/Game/WesTurner_Character/Particles/P_Explosion.P_Explosion" _returnvalue)
  (Audio|SpawnSoundatLocation "/Game/assets/SoundFX/Sound_Cues/explosion.explosion" _returnvalue)
  (Game|Damage|ApplyRadialDamage (Variables|Default|GetExplosionDamage) (Transformation|GetActorLocation) (Variables|Default|GetExplosionDamageRadius) "/Script/Engine.DamageType" 0 self 0 true "ECC_Visibility")
  (Actor|DestroyActor))

(fn ConstructionScript)